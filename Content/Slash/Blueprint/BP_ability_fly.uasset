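; BP_ability_fly is an ability actor that flies a slash Niagara effect forward in a straight line.
; On BeginPlay it records its location and an end point a fixed distance along its forward vector, then plays a timeline that lerps the actor between them without sweeping.
; The construction script applies the NESlash system and relative offset to the Niagara component.
; The graph contains no hit or overlap logic.
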(event Custom|Ability
  (bind _alpha (Timeline|时间轴 PlayFromStart)
    (:Update
      (Transformation|SetActorLocation self (Math|Vector|Lerp(Vector) (Variables|Default|Getlocation_began) (Variables|Default|Getlocation_end) _alpha) false false))))

(event EventBeginPlay
  (bind _returnvalue (Transformation|GetActorLocation))
  (Variables|Default|Setlocation_began _returnvalue)
  (Variables|Default|Setlocation_end (+ _returnvalue (* (Transformation|GetActorForwardVector) 8e+02)))
  (CallFunction|Ability))

(event Collision|EventActorBeginOverlap
  (params (OtherActor :type Actor%20Object%20Reference)))

(event EventTick
  (params (DeltaSeconds :type Float%20%28single-precision%29)))

(fn ConstructionScript
  (Class|NiagaraComponent|SetAsset (Variables|Default|GetNiagara) (Variables|Default|GetNE_slash) true)
  (Transformation|SetRelativeLocation (Variables|Default|GetNiagara) (Variables|Default|GetLaction) false false))