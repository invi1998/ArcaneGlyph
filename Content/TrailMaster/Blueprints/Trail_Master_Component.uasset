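; Trail Master component that spawns Trail_Core actors at the owner's static and skeletal mesh components tagged "Trail", leaving a mesh-based trail.
; StartTrail and StopTrail open and close a gate on Tick, whose Delay throttles spawning to a fixed or randomized interval from TrailData.
; SpawnOnce enters the same delayed path, bypassing the gate.
; Each Trail_Core receives its source mesh and TrailData, which has an empty OnRep.
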(event Custom|Start%20Trail
  (bind _trail_data (Variables|TrailMaster|GetTrail%20Data))
  (bind ___spawngroup__ (Utilities|Struct|BreakTrailData _trail_data))
  (bind (_trailspawninterval _randomizespawninterval) (Utilities|Struct|BreakSpawnGroup ___spawngroup__))
  ;[1 1 1] Start and Stop events
  (Utilities|FlowControl|Gate true) ; enters at Open
)

(event Custom|Stop%20Trail
  (bind _trail_data (Variables|TrailMaster|GetTrail%20Data))
  (bind ___spawngroup__ (Utilities|Struct|BreakTrailData _trail_data))
  (bind (_trailspawninterval _randomizespawninterval) (Utilities|Struct|BreakSpawnGroup ___spawngroup__))
  ;[1 1 1] Start and Stop events
  (Utilities|FlowControl|Gate true) ; enters at Close
)

(event Custom|Spawn%20Once
  (bind _trail_data (Variables|TrailMaster|GetTrail%20Data))
  (bind ___spawngroup__ (Utilities|Struct|BreakTrailData _trail_data))
  (bind (_trailspawninterval _randomizespawninterval) (Utilities|Struct|BreakSpawnGroup ___spawngroup__))
  (Utilities|FlowControl|Delay (select _randomizespawninterval (Math|Random|RandomFloatinRange 0.0 _trailspawninterval) _trailspawninterval))
  (for _array_element (Actor|GetComponentsbyTag (Components|GetOwner) "/Script/Engine.ActorComponent" "Trail")
    (Utilities|FlowControl|Sequence
      (:then_0
        (bind _as静态网格体组件 (Utilities|Casting|CastToStaticMeshComponent _array_element))
        (Game|SpawnActorfromClass "/Game/TrailMaster/Blueprints/Trail_Core.Trail_Core_C" (Transformation|GetWorldTransform _as静态网格体组件) "AlwaysSpawn" "OverrideRootScale" 0 _as静态网格体组件 0 "NewEnumerator0" (Variables|TrailMaster|GetTrail%20Data) 0 :!pinned true) ; Spawn Trail for a Static Mesh
      )
      (:then_1
        (bind _as骨骼网格体组件 (Utilities|Casting|CastToSkeletalMeshComponent _array_element))
        (Game|SpawnActorfromClass "/Game/TrailMaster/Blueprints/Trail_Core.Trail_Core_C" (Transformation|GetWorldTransform _as骨骼网格体组件) "AlwaysSpawn" "OverrideRootScale" 0 0 _as骨骼网格体组件 "NewEnumerator1" (Variables|TrailMaster|GetTrail%20Data) 0 :!pinned true) ; Spawn Trail for a Skeletal Mesh
      ))))

(event EventTick
  (params (DeltaSeconds :type Float%20%28single-precision%29))
  (bind _trail_data (Variables|TrailMaster|GetTrail%20Data))
  (bind ___spawngroup__ (Utilities|Struct|BreakTrailData _trail_data))
  (bind (_trailspawninterval _randomizespawninterval) (Utilities|Struct|BreakSpawnGroup ___spawngroup__))
  (Utilities|FlowControl|Gate true
    (:Exit
      (Utilities|FlowControl|Delay (select _randomizespawninterval (Math|Random|RandomFloatinRange 0.0 _trailspawninterval) _trailspawninterval))
      (for _array_element (Actor|GetComponentsbyTag (Components|GetOwner) "/Script/Engine.ActorComponent" "Trail")
        (Utilities|FlowControl|Sequence
          (:then_0
            (bind _as静态网格体组件 (Utilities|Casting|CastToStaticMeshComponent _array_element))
            (Game|SpawnActorfromClass "/Game/TrailMaster/Blueprints/Trail_Core.Trail_Core_C" (Transformation|GetWorldTransform _as静态网格体组件) "AlwaysSpawn" "OverrideRootScale" 0 _as静态网格体组件 0 "NewEnumerator0" (Variables|TrailMaster|GetTrail%20Data) 0 :!pinned true) ; Spawn Trail for a Static Mesh
          )
          (:then_1
            (bind _as骨骼网格体组件 (Utilities|Casting|CastToSkeletalMeshComponent _array_element))
            (Game|SpawnActorfromClass "/Game/TrailMaster/Blueprints/Trail_Core.Trail_Core_C" (Transformation|GetWorldTransform _as骨骼网格体组件) "AlwaysSpawn" "OverrideRootScale" 0 0 _as骨骼网格体组件 "NewEnumerator1" (Variables|TrailMaster|GetTrail%20Data) 0 :!pinned true) ; Spawn Trail for a Skeletal Mesh
          ))))))

(fn OnRepTrailData)