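; Trail ghost actor that leaves a fading afterimage of a source static or skeletal mesh, then destroys itself after its lifetime.
; On BeginPlay it clones the static mesh or copies the skeletal pose into a PoseableMesh, applying a dynamic trail material to every slot.
; After a spawn delay, a gated Tick turns age into a 0-1 alpha driving scale, opacity, color and translucent sort priority, plus a per-tick offset.
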(event Custom|Open%20Gate
  (bind _returnvalue (Actor|GetGameTimeSinceCreation))
  (bind _trail_data (Variables|Default|GetTrail%20Data))
  (bind ___spawngroup__ (Utilities|Struct|BreakTrailData _trail_data))
  (bind (_spawndelay _lifetime) (Utilities|Struct|BreakSpawnGroup ___spawngroup__))
  (bind _returnvalue_2 (- _returnvalue _spawndelay))
  (Utilities|FlowControl|Gate true) ; enters at Open
)

(event Custom|Event%20Fire
  (CallFunction|OpenGate :!pinned true) ; Fires "Update Group" Gate Tick
  (switch Utilities|FlowControl|Switch|SwitchonSwitchClass (Variables|Default|GetSwitch%20Class)
    (:NewEnumerator0
      ;[1 1 1] Makes mesh visible again
      (Development|SetHiddeninGame (Variables|Components|GetTrail%20Static%20Mesh%20) false false))
    (:NewEnumerator1
      (Development|SetHiddeninGame (Variables|Components|GetTrail%20Skeletal%20Mesh) false false))))

(event EventBeginPlay
  ;[1 1 1] Static Mesh or Skeletal Mesh Switch
  (switch Utilities|FlowControl|Switch|SwitchonSwitchClass (Variables|Default|GetSwitch%20Class)
    (:NewEnumerator0
      (CallFunction|CloneStaticMeshfromSource :!pinned true) ; Gets a copy of given Static Mesh
    )
    (:NewEnumerator1
      (CallFunction|PoseSkeletalMeshfromSource :!pinned true) ; Gets a copy of given Skeletal Mesh
    ))
  (CallFunction|SetMaterialSlotsOfCloneMesh :!pinned true) ; Replaces all materials of given mesh with Trail Mat.
  ;[1 1 1] Wait for the given spawn delay
  (Utilities|Time|SetTimerbyEvent (delegate Custom|Event%20Fire) (+ (Utilities|Struct|BreakSpawnGroup (Utilities|Struct|BreakTrailData (Variables|Default|GetTrail%20Data))) 1e-05)))

(event EventTick
  (params (DeltaSeconds :type Float%20%28single-precision%29))
  (bind _returnvalue (Actor|GetGameTimeSinceCreation))
  (bind _trail_data (Variables|Default|GetTrail%20Data))
  (bind ___spawngroup__ (Utilities|Struct|BreakTrailData _trail_data))
  (bind (_spawndelay _lifetime) (Utilities|Struct|BreakSpawnGroup ___spawngroup__))
  (bind _returnvalue_2 (- _returnvalue _spawndelay))
  (Utilities|FlowControl|Gate true
    (:Exit
      ;[1 1 1] Calculate Lifetime and Alpha.
      (if (> _returnvalue_2 _lifetime)
        ;;[1 0 0] Destroys itself when reach given Lifetime
        (Actor|DestroyActor)
        (else
          ;;[0 1 0.0488] 0-1 Alpha for Lerp Functions
          (Variables|Default|SetAlpha (Math|Float|NormalizetoRange _returnvalue_2 0.0 _lifetime))
          (CallFunction|SetMeshDrawPriority :!pinned true) ; For Transculent Materials. Sorts render priority
          (CallFunction|TrailScaleLerp :!pinned true) ; Mesh Scale Function
          (CallFunction|TrailOpacityLerp :!pinned true) ; Opacity Fade-Out Fuction
          (CallFunction|TrailColorLerp :!pinned true) ; Color Function
          (CallFunction|AddOffset :!pinned true) ; Offset Function
        )))))

(fn ConstructionScript)

(fn CloneStaticMeshfromSource
  (bind _returnvalue (Transformation|GetActorTransform))
  (bind _static_mesh_ref (Variables|Components|GetStatic%20Mesh%20Ref))
  (Utilities|IsValid _static_mesh_ref
    (:Is%20Valid
      (bind _returnvalue_2 (AddComponent|AddStaticMeshComponent true (Math|Transform|MakeTransform (.location _returnvalue) (.rotation _returnvalue) (- (.scale (Transformation|GetWorldTransform _static_mesh_ref)) "0.010000,0.010000,0.010000")) :!pinned true)) ; Mesh should be Hidden in Game. Later will be visible again.
      (bind _output_get (Variables|Components|SetTrail%20Static%20Mesh%20 _returnvalue_2))
      (Variables|Default|SetTrail%20Mesh%20Transform (Transformation|GetWorldTransform _returnvalue_2))
      (Components|StaticMesh|SetStaticMesh _output_get (Variables|/Script/Engine.StaticMeshComponent|GetStaticMesh _static_mesh_ref)))
    (:Is%20Not%20Valid
      (Actor|DestroyActor))))

(fn SetMaterialSlotsOfCloneMesh
  (bind _trail_static_mesh_ (Variables|Components|GetTrail%20Static%20Mesh%20))
  (bind _trail_skeletal_mesh (Variables|Components|GetTrail%20Skeletal%20Mesh))
  (bind _switch_class (Variables|Default|GetSwitch%20Class))
  (bind _returnvalue (Utilities|Select :Index _switch_class :NewEnumerator0 _trail_static_mesh_ :NewEnumerator1 _trail_skeletal_mesh))
  ;[1 1 1] Create New Material Instance
  (bind _returnvalue_2 (Rendering|Material|CreateDynamicMaterialInstance (Utilities|Struct|BreakMaterialGroup (Utilities|Struct|BreakTrailData (Variables|Default|GetTrail%20Data))) "None" :!class /Script/Engine.KismetMaterialLibrary))
  (bind _output_get (Variables|Default|SetMaterial%20Instance _returnvalue_2))
  ;[1 1 1] Material Emissive Multiplier Parameter
  (Rendering|Material|SetScalarParameterValue _output_get "Emissive Multiply" (Utilities|Struct|BreakColorGroup (Utilities|Struct|BreakTrailData (Variables|Default|GetTrail%20Data))) :!class /Script/Engine.MaterialInstanceDynamic)
  (CallFunction|MaterialLinearStartColor :!pinned true) ; Material Color Parameter
  ;[1 1 1] Material Fresnel Parameter
  (Rendering|Material|SetScalarParameterValue (Variables|Default|GetMaterial%20Instance) "Fresnel" (Utilities|Struct|BreakMaterialGroup (Utilities|Struct|BreakTrailData (Variables|Default|GetTrail%20Data))) :!class /Script/Engine.MaterialInstanceDynamic)
  (Utilities|IsValid (Utilities|Select :Index (Variables|Default|GetSwitch%20Class) :NewEnumerator0 (Variables|Components|GetTrail%20Static%20Mesh%20) :NewEnumerator1 (Variables|Components|GetTrail%20Skeletal%20Mesh))
    (:Is%20Valid
      ;[1 1 1] Replace all material slots of reference mesh with Trail Material.
      (for (_ _array_index) (Rendering|Material|GetMaterials _returnvalue)
        (Rendering|Material|SetMaterial _returnvalue _array_index (Variables|Default|GetMaterial%20Instance))))))

(fn TrailScaleLerp
  (bind _trail_data (Variables|Default|GetTrail%20Data))
  (bind ___updategroup__ (Utilities|Struct|BreakTrailData _trail_data))
  (bind (_usecustomscale _targetscaleovertime) (Utilities|Struct|BreakUpdateGroup ___updategroup__))
  (Transformation|SetWorldScale3D (Utilities|Select :Index (Variables|Default|GetSwitch%20Class) :NewEnumerator0 (Variables|Components|GetTrail%20Static%20Mesh%20) :NewEnumerator1 (Variables|Components|GetTrail%20Skeletal%20Mesh)) (Math|Vector|Lerp(Vector) (.scale (Variables|Default|GetTrail%20Mesh%20Transform)) (select _usecustomscale _targetscaleovertime (.scale (Variables|Default|GetTrail%20Mesh%20Transform))) (Variables|Default|GetAlpha))))

(fn TrailOpacityLerp
  (if (Utilities|Struct|BreakMaterialGroup (Utilities|Struct|BreakTrailData (Variables|Default|GetTrail%20Data)))
    (Rendering|Material|SetScalarParameterValue (Variables|Default|GetMaterial%20Instance) "Opacity" (Math|Float|Lerp 1.0 0.0 (Variables|Default|GetAlpha)) :!class /Script/Engine.MaterialInstanceDynamic)))

(fn TrailColorLerp
  (bind _trail_data (Variables|Default|GetTrail%20Data))
  (bind _trail_data_2 (Variables|Default|GetTrail%20Data))
  (bind ___colorgroup__ (Utilities|Struct|BreakTrailData _trail_data))
  (bind ___colorgroup___2 (Utilities|Struct|BreakTrailData _trail_data_2))
  (bind _curvelinearcolor (Utilities|Struct|BreakColorGroup ___colorgroup__))
  (bind (_from _to _usecurvecolor) (Utilities|Struct|BreakColorGroup ___colorgroup___2))
  (if _usecurvecolor
    ;[1 1 1] Linear Curve Color
    (Rendering|Material|SetVectorParameterValue (Variables|Default|GetMaterial%20Instance) "Color" (Math|Curves|GetLinearColorValue _curvelinearcolor (* (.MaxTime (Math|Curves|GetTimeRange _curvelinearcolor)) (Variables|Default|GetAlpha))) :!class /Script/Engine.MaterialInstanceDynamic)
    (else
      (Rendering|Material|SetVectorParameterValue (Variables|Default|GetMaterial%20Instance) "Color" (Math|Color|Lerp(LinearColor) _from _to (Variables|Default|GetAlpha)) :!class /Script/Engine.MaterialInstanceDynamic))))

(fn AddOffset
  (Transformation|AddWorldOffset (Utilities|Select :Index (Variables|Default|GetSwitch%20Class) :NewEnumerator0 (Variables|Components|GetTrail%20Static%20Mesh%20) :NewEnumerator1 (Variables|Components|GetTrail%20Skeletal%20Mesh)) (Utilities|Struct|BreakUpdateGroup (Utilities|Struct|BreakTrailData (Variables|Default|GetTrail%20Data))) true false))

(fn SetMeshDrawPriority
  (Rendering|SetTranslucentSortPriority (Utilities|Select :Index (Variables|Default|GetSwitch%20Class) :NewEnumerator0 (Variables|Components|GetTrail%20Static%20Mesh%20) :NewEnumerator1 (Variables|Components|GetTrail%20Skeletal%20Mesh)) (Math|Float|Truncate (* (Variables|Default|GetAlpha) 1e+02))))

(fn PoseSkeletalMeshfromSource
  (bind _skeletal_mesh_ref (Variables|Components|GetSkeletal%20Mesh%20Ref))
  (bind _returnvalue (Transformation|GetWorldTransform _skeletal_mesh_ref))
  (bind _returnvalue_2 (AddComponent|AddPoseableMeshComponent true (Math|Transform|MakeTransform (.location _returnvalue) (.rotation _returnvalue) (- (.scale _returnvalue) "0.010000,0.010000,0.010000"))))
  (Class|SkinnedMeshComponent|SetSkeletalMesh _returnvalue_2 (Variables|/Script/Engine.SkinnedMeshComponent|GetSkeletalMesh _skeletal_mesh_ref) true)
  (bind _output_get (Variables|Components|SetTrail%20Skeletal%20Mesh _returnvalue_2))
  (Class|PoseableMeshComponent|CopyPosefromSkeletalComponent _output_get _skeletal_mesh_ref))

(fn MaterialLinearStartColor
  (bind _trail_data (Variables|Default|GetTrail%20Data))
  (bind _material_instance (Variables|Default|GetMaterial%20Instance))
  (bind ___colorgroup__ (Utilities|Struct|BreakTrailData _trail_data))
  (bind (_from _usecurvecolor _curvelinearcolor) (Utilities|Struct|BreakColorGroup ___colorgroup__))
  (if _usecurvecolor
    (Rendering|Material|SetVectorParameterValue _material_instance "Color" (Math|Curves|GetLinearColorValue _curvelinearcolor 0.0) :!class /Script/Engine.MaterialInstanceDynamic)
    (else
      (Rendering|Material|SetVectorParameterValue _material_instance "Color" _from :!class /Script/Engine.MaterialInstanceDynamic))))