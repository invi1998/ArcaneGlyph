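; Test actor for the TrailMaster demo room that starts a TrailMasterComponent trail on BeginPlay.
; With Rotate set, Tick spins every static mesh component tagged "Trail".
; The construction script either adds a RotatingMovementComponent for Spin or activates the MoveFWBW timeline, whose update eases the mesh between two target locations.
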(event EventBeginPlay
  (Default|StartTrail (Variables|Components|GetTrail_Master_Component))
  (Variables|Default|SetStart%20Transform (Transformation|GetActorTransform))
  (Components|Activation|SetAutoActivate (Variables|Default|GetMove%20FW/BW) true))

(event EventTick
  (params (DeltaSeconds :type Float%20%28single-precision%29))
  (if (Variables|Default|GetRotate)
    (for _array_element (Actor|GetComponentsbyTag "/Script/Engine.StaticMeshComponent" "Trail")
      (Transformation|AddWorldRotation _array_element (Variables|Default|GetAdd%20World%20Rotation) false false))))

(fn ConstructionScript
  (bind _move_fw_bw (Variables|Default|GetMove%20FW/BW))
  (if (Variables|Default|GetSpin)
    (bind _returnvalue (AddComponent|AddRotatingMovementComponent))
    (Variables|/Script/Engine.RotatingMovementComponent|SetRotationRate _returnvalue (Variables|Default|GetRotation%20Rate))
    (Variables|/Script/Engine.RotatingMovementComponent|SetPivotTranslation _returnvalue (Variables|Default|GetPivot%20Translation))
    (else
      (Components|Activation|SetAutoActivate _move_fw_bw true)
      (Audio|Components|Audio|Play _move_fw_bw))))

(fn NewFunction0
  (Transformation|SetActorLocation "0, 0, 0" false false))