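; Spear weapon Blueprint for the Sparta weapon set that shows the current Spark level through glowing material colors and a VFX burst.
; Both light parameters on the skeletal mesh start black at BeginPlay.
; OnSparkChanged ignores unchanged values, then maps levels zero to four to HDR colors on those parameters.
; When Spark increases, it also spawns the Sacura cast Niagara effect attached at the mesh's Root.
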(event EventBeginPlay
  (|CallParentFunction)
  (Rendering|Material|SetColorParameterValueonMaterials :self (Variables|Default|GetWeaponSkeletalMesh) :ParameterName "Light1")
  (Rendering|Material|SetColorParameterValueonMaterials :self (Variables|Default|GetWeaponSkeletalMesh) :ParameterName "Light2"))

(event Collision|EventActorBeginOverlap
  (params (OtherActor :type Actor%20Object%20Reference))
  (|CallParentFunction OtherActor) ; 此节点被禁用，将不会被调用。\n从引脚连出引线来编译功能。
)

(event EventTick
  (params (DeltaSeconds :type Float%20%28single-precision%29))
  (|CallParentFunction DeltaSeconds) ; 此节点被禁用，将不会被调用。\n从引脚连出引线来编译功能。
)

(event EventOnSparkChanged
  (params (InSparkValue :type Integer))
  (if (not (== (Variables|Default|GetPre%20Spark%20Value) InSparkValue))
    (Variables|Default|SetIsSparkAdd (> InSparkValue (Variables|Default|GetPre%20Spark%20Value)))
    (bind _output_get (Variables|Default|SetPre%20Spark%20Value InSparkValue))
    (Utilities|FlowControl|Sequence
      (:then_0
        (switch int _output_get
          (:0
            (Rendering|Material|SetColorParameterValueonMaterials :self (Variables|Default|GetWeaponSkeletalMesh) :ParameterName "Light1")
            (Rendering|Material|SetColorParameterValueonMaterials :self (Variables|Default|GetWeaponSkeletalMesh) :ParameterName "Light2"))
          (:1
            (Rendering|Material|SetColorParameterValueonMaterials (Variables|Default|GetWeaponSkeletalMesh) "Light1" "(R=9202.320312,G=10000.000000,B=9345.417969,A=1.000000)")
            (Rendering|Material|SetColorParameterValueonMaterials (Variables|Default|GetWeaponSkeletalMesh) "Light2" "(R=10000.000000,G=0.000000,B=0.000000,A=1.000000)"))
          (:2
            (Rendering|Material|SetColorParameterValueonMaterials (Variables|Default|GetWeaponSkeletalMesh) "Light1" "(R=2708.634033,G=5292.634277,B=10000.000000,A=1.000000)")
            (Rendering|Material|SetColorParameterValueonMaterials (Variables|Default|GetWeaponSkeletalMesh) "Light2" "(R=10000.000000,G=0.000000,B=0.000000,A=1.000000)"))
          (:3
            (Rendering|Material|SetColorParameterValueonMaterials (Variables|Default|GetWeaponSkeletalMesh) "Light1" "(R=2667.786377,G=10000.000000,B=7457.710449,A=1.000000)")
            (Rendering|Material|SetColorParameterValueonMaterials (Variables|Default|GetWeaponSkeletalMesh) "Light2" "(R=10000.000000,G=0.000000,B=0.000000,A=1.000000)"))
          (:4
            (Rendering|Material|SetColorParameterValueonMaterials (Variables|Default|GetWeaponSkeletalMesh) "Light1" "(R=10000.000000,G=1053.881592,B=2939.212891,A=1.000000)")
            (Rendering|Material|SetColorParameterValueonMaterials (Variables|Default|GetWeaponSkeletalMesh) "Light2" "(R=10000.000000,G=0.000000,B=0.000000,A=1.000000)"))))
      (:then_1
        (if (Variables|Default|GetIsSparkAdd)
          (Niagara|SpawnSystemAttached "/Game/WizardSpellsPack/Effects/NS_Sacura_cast.NS_Sacura_cast" (Variables|Default|GetWeaponSkeletalMesh) "Root" "0, 0, 0" "0, 0, 0" "KeepRelativeOffset" true))))))

(fn ConstructionScript
  (|CallParentFunction))