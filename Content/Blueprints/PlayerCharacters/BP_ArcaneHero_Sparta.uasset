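; Player hero character Blueprint for Sparta that shows floating combat text when it deals damage and opens the pause screen.
; BeginPlay spawns and initialises a BP_CombatText actor, then binds to the HeroCombatComponent damage event to show normal or critical numbers at the impact point.
; ActivateCombatText also supports status, damage-reduction, elemental and damage-taken styles via type and subtype switches, though only normal and critical are triggered here.
; The pause input pushes a tag-resolved soft widget onto the HUD stack.
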(event Custom|OnCauseDamageShowFloatText
  (params (InHitImpactLocation :type Vector) (InDamageValue :type Integer) (bIsCriticalHit :type Boolean))
  (CallFunction|ActivateCombatText (select bIsCriticalHit "NewEnumerator1" "NewEnumerator0") 0 (Math|Conversions|ToFloat(Integer) InDamageValue) InHitImpactLocation))

(event Input|EnhancedActionEvents|EnhancedInputActionIA_PauseGame
  (params (ActionValue :type Boolean) (ElapsedSeconds :type Float%20%28double-precision%29) (TriggeredSeconds :type Float%20%28double-precision%29) (InputAction :type Input%20Action%20Object%20Reference :default "/Game/Blueprints/PlayerCharacters/Input/Actions/IA_PauseGame.IA_PauseGame"))
  (:Started
    (|PushSoftWidget (Game|GetPlayerController 0) (Class|ArcaneBlueprintFunctionLibrary|GetFrontendSoftWidgetClassbyTag "(TagName=\"Frontend.Widget.HUD.PauseScreen\")") "(TagName=\"Frontend.WidgetStack.HUD\")" true)))

(event EventBeginPlay
  (bind _returnvalue (Game|SpawnActorfromClass "/Game/DynamicCombatText/Blueprints/BP_CombatText.BP_CombatText_C" (Math|Transform|MakeTransform "0, 0, 0") "Undefined" "OverrideRootScale" 0 0))
  (bind _output_get (Variables|Default|SetCombatText _returnvalue))
  (Default|Initialise _output_get self "0, 0,175.000000")
  (EventDispatchers|AssignOnCauseDamage (Variables|Default|GetHeroCombatComponent) (delegate Custom|OnCauseDamageShowFloatText)))

(event Collision|EventActorBeginOverlap
  (params (OtherActor :type Actor%20Object%20Reference)))

(event EventTick
  (params (DeltaSeconds :type Float%20%28single-precision%29)))

(fn ConstructionScript)

(fn ActivateCombatText
  (params (TextType :type ENUM_TextTypes%20Enum :default "NewEnumerator0") (TextSubTypeIndex :type Integer) (Damage :type Float%20%28double-precision%29) (ImpactPoint :type Vector))
  (LocalVariables|SetTextType_Local TextType)
  (LocalVariables|SetTextSubType_Local TextSubTypeIndex)
  (LocalVariables|SetDamage_Local Damage)
  (LocalVariables|SetImpactPoint_Local ImpactPoint)
  (switch Utilities|FlowControl|Switch|SwitchonENUM_TextTypes (LocalVariables|GetTextType_Local)
    (:NewEnumerator0
      ;[1 1 1] Normal damage
      (Default|ActivateText (Variables|Default|GetCombatText) "NewEnumerator0" (LocalVariables|GetDamage_Local) true (LocalVariables|GetImpactPoint_Local)))
    (:NewEnumerator1
      ;[1 1 1] Critical Hit Damage
      (Default|ActivateText (Variables|Default|GetCombatText) "NewEnumerator1" (LocalVariables|GetDamage_Local) true (LocalVariables|GetImpactPoint_Local)))
    (:NewEnumerator14
      (switch int (LocalVariables|GetTextSubType_Local)
        (:0
          ;[1 1 1] Stun
          (Default|ActivateTextwithOverrides (Variables|Default|GetCombatText) "NewEnumerator14" 0.0 true (LocalVariables|GetImpactPoint_Local) true "STUN" true "(R=0.786458,G=0.050748,B=0.144906,A=1.000000)" false 0 true "(R=0.062500,G=0.005825,B=0.007692,A=1.000000)" false "(R=0.000000,G=0.000000,B=0.000000,A=1.000000)"))
        (:1
          ;[1 1 1] Slow
          (Default|ActivateTextwithOverrides (Variables|Default|GetCombatText) "NewEnumerator14" 0.0 true (LocalVariables|GetImpactPoint_Local) true "SLOW" true "(R=0.921875,G=0.683376,B=0.045696,A=1.000000)" false 0 true "(R=0.083333,G=0.067189,B=0.004680,A=1.000000)" false "(R=0.000000,G=0.000000,B=0.000000,A=1.000000)"))
        (:2
          ;[1 1 1] Silence
          (Default|ActivateTextwithOverrides (Variables|Default|GetCombatText) "NewEnumerator14" 0.0 true (LocalVariables|GetImpactPoint_Local) true "SILENCE" true "(R=0.044310,G=0.305868,B=0.468750,A=1.000000)" false 0 true "(R=0.011227,G=0.052698,B=0.067708,A=1.000000)" false "(R=0.000000,G=0.000000,B=0.000000,A=1.000000)"))
        (:3
          ;[1 1 1] Confuse
          (Default|ActivateTextwithOverrides (Variables|Default|GetCombatText) "NewEnumerator14" 0.0 true (LocalVariables|GetImpactPoint_Local) true "CONFUSE" true "(R=0.927083,G=0.018852,B=0.693504,A=1.000000)" false 0 true "(R=0.055738,G=0.007898,B=0.057292,A=1.000000)" false "(R=0.000000,G=0.000000,B=0.000000,A=1.000000)"))))
    (:NewEnumerator21
      (switch int (LocalVariables|GetTextSubType_Local)
        (:0
          ;[1 1 1] Block
          (Default|ActivateTextwithOverrides (Variables|Default|GetCombatText) "NewEnumerator21" 0.0 true (LocalVariables|GetImpactPoint_Local) true "BLOCK" false "(R=0.000000,G=0.000000,B=0.000000,A=1.000000)" false 0 false "(R=0.000000,G=0.000000,B=0.000000,A=1.000000)" false "(R=0.000000,G=0.000000,B=0.000000,A=1.000000)"))
        (:1
          ;[1 1 1] Evade
          (Default|ActivateTextwithOverrides (Variables|Default|GetCombatText) "NewEnumerator21" 0.0 true (LocalVariables|GetImpactPoint_Local) true "EVADE" false "(R=0.000000,G=0.000000,B=0.000000,A=1.000000)" false 0 false "(R=0.000000,G=0.000000,B=0.000000,A=1.000000)" false "(R=0.000000,G=0.000000,B=0.000000,A=1.000000)"))
        (:2
          ;[1 1 1] Parry
          (Default|ActivateTextwithOverrides (Variables|Default|GetCombatText) "NewEnumerator21" 0.0 true (LocalVariables|GetImpactPoint_Local) true "PARRY" false "(R=0.000000,G=0.000000,B=0.000000,A=1.000000)" false 0 false "(R=0.000000,G=0.000000,B=0.000000,A=1.000000)" false "(R=0.000000,G=0.000000,B=0.000000,A=1.000000)"))
        (:3
          ;[1 1 1] Absorb
          (Default|ActivateTextwithOverrides (Variables|Default|GetCombatText) "NewEnumerator21" 0.0 true (LocalVariables|GetImpactPoint_Local) true "ABSORB" false "(R=0.000000,G=0.000000,B=0.000000,A=1.000000)" false 0 false "(R=0.000000,G=0.000000,B=0.000000,A=1.000000)" false "(R=0.000000,G=0.000000,B=0.000000,A=1.000000)"))))
    (:NewEnumerator23
      (switch int (LocalVariables|GetTextSubType_Local)
        (:0
          ;[1 1 1] Fire
          (Default|ActivateTextwithOverrides (Variables|Default|GetCombatText) "NewEnumerator23" (LocalVariables|GetDamage_Local) true (LocalVariables|GetImpactPoint_Local) true "Burn" true "(R=0.692708,G=0.234298,B=0.030984,A=1.000000)" true "/Game/DynamicCombatText/Textures/T_FireIcon.T_FireIcon" false "(R=0.000000,G=0.000000,B=0.000000,A=1.000000)" false "(R=0.000000,G=0.000000,B=0.000000,A=1.000000)"))
        (:1
          ;[1 1 1] Poison
          (Default|ActivateTextwithOverrides (Variables|Default|GetCombatText) "NewEnumerator23" (LocalVariables|GetDamage_Local) true (LocalVariables|GetImpactPoint_Local) true "Poison" true "(R=0.037627,G=0.692708,B=0.250169,A=1.000000)" true "/Game/DynamicCombatText/Textures/T_PoisonIcon.T_PoisonIcon" false "(R=0.000000,G=0.000000,B=0.000000,A=1.000000)" false "(R=0.000000,G=0.000000,B=0.000000,A=1.000000)"))
        (:2
          ;[1 1 1] Cold
          (Default|ActivateTextwithOverrides (Variables|Default|GetCombatText) "NewEnumerator23" (LocalVariables|GetDamage_Local) true (LocalVariables|GetImpactPoint_Local) true "Cold" true "(R=0.013630,G=0.500073,B=0.833333,A=1.000000)" true "/Game/DynamicCombatText/Textures/T_IceIcon.T_IceIcon" false "(R=0.000000,G=0.000000,B=0.000000,A=1.000000)" false "(R=0.000000,G=0.000000,B=0.000000,A=1.000000)"))
        (:3
          ;[1 1 1] Electric
          (Default|ActivateTextwithOverrides (Variables|Default|GetCombatText) "NewEnumerator23" (LocalVariables|GetDamage_Local) true (LocalVariables|GetImpactPoint_Local) true "Shock" true "(R=0.692708,G=0.586732,B=0.209256,A=1.000000)" true "/Game/DynamicCombatText/Textures/T_LightningIcon.T_LightningIcon" false "(R=0.000000,G=0.000000,B=0.000000,A=1.000000)" false "(R=0.000000,G=0.000000,B=0.000000,A=1.000000)"))))
    (:NewEnumerator24
      ;[1 1 1] Player Hit Damage
      (Default|ActivateText (Variables|Default|GetCombatText) "NewEnumerator24" (LocalVariables|GetDamage_Local) true (LocalVariables|GetImpactPoint_Local)))))