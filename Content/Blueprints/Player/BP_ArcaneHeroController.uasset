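; BP_ArcaneHeroController is the hero's player controller, setting up CommonUI and input registration when the loading screen deactivates.
; It adds the primary layout widget to the viewport and registers it with the frontend UI subsystem.
; In an Arcane game mode it activates the HUD-drawing ability by tag; otherwise it pushes the press-any-key screen.
; It also registers gameplay mapping contexts with Enhanced Input user settings.
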(event EventBeginPlay)

(event EventTick
  (params (DeltaSeconds :type Float%20%28single-precision%29)))

(event EventPossess
  (params (PossessedPawn :type Pawn%20Object%20Reference)))

(event EventOnLoadingScreenDeactivated
  (bind _returnvalue (Subsystems|GetFrontendUISubsystem))
  (bind _returnvalue_2 (PlayerController|LocalPlayerSubsystems|GetEnhancedInputLocalPlayerSubsystem))
  (bind _returnvalue_3 (Class|EnhancedInputSubsystemInterface|GetUserSettings _returnvalue_2))
  (Utilities|FlowControl|Sequence
    (:then_0
      (bind _returnvalue_4 (UserInterface|CreateWidget "/Game/Blueprints/UI/Widgets/Menu/WBP_CUW_PrimaryLayout.WBP_CUW_PrimaryLayout_C" self))
      (UserInterface|Viewport|AddtoViewport _returnvalue_4 0)
      (Utilities|IsValid _returnvalue
        (:Is%20Valid
          (Class|FrontendUISubsystem|RegisterCreatedPrimaryLayoutWidget _returnvalue _returnvalue_4)
          (Utilities|Casting|CastToArcaneGameModeBase (Game|GetGameMode)
            (:then
              (Class|ArcaneAbilitySystemComponent|TryActivateAbilitybyTag (Class|ArcaneBlueprintFunctionLibrary|GetArcaneASCfromActor (Game|GetPlayerCharacter 0)) "(TagName=\"InputTag.DrawCommonUIHUD\")"))
            (:CastFailed
              (|PushSoftWidget self (Class|ArcaneBlueprintFunctionLibrary|GetFrontendSoftWidgetClassbyTag "(TagName=\"Frontend.Widget.Frontend.PressAnyKeyScreen\")") "(TagName=\"Frontend.WidgetStack.Frontend\")" true))))))
    (:then_1
      (Class|EnhancedInputUserSettings|RegisterInputMappingContext _returnvalue_3 "/Game/Blueprints/PlayerCharacters/Input/IMC_Default.IMC_Default")
      (Class|EnhancedInputUserSettings|RegisterInputMappingContext _returnvalue_3 "/Game/Blueprints/PlayerCharacters/Input/IMC_Spear.IMC_Spear")
      (Class|EnhancedInputUserSettings|RegisterInputMappingContext _returnvalue_3 "/Game/Blueprints/PlayerCharacters/Input/IMC_PickUpHeal.IMC_PickUpHeal")
      (Class|EnhancedInputUserSettings|RegisterInputMappingContext _returnvalue_3 "/Game/Blueprints/PlayerCharacters/Input/IMC_PickUpRage.IMC_PickUpRage")
      (Class|EnhancedInputUserSettings|RegisterInputMappingContext _returnvalue_3 "/Game/Blueprints/PlayerCharacters/Input/IMC_TargetLock.IMC_TargetLock"))))

(fn ConstructionScript)