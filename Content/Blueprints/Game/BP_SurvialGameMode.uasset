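; Survival game mode Blueprint that plays looping music and handles the presentation and outcome of wave-based runs.
; It reacts to state-change events by showing wave text or countdown widgets, flagging the final wave and overriding its enemy spawn delay.
; Completing all waves saves the next difficulty unlock based on the saved one.
; Victory and death both fade out, pause, and push modals offering replay, main menu or quit, loading levels by gameplay tag.
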(event Custom|OnSurvialGameModeStateChangedEvent
  (params (state :type EArcaneSurvialGameModeState%20Enum :default "WaitSpawnNewWave"))
  (switch Utilities|FlowControl|Switch|SwitchonEArcaneSurvialGameModeState state
    (:WaitSpawnNewWave
      (CallFunction|CreateWaveWidgetCountDown "新的波次即将来袭" (Variables|Default|GetSpawnNewWaveWaitTime)))
    (:SpawningNewWave
      (CallFunction|CreateWaveWidget (Utilities|Text|FormatText "当前来袭波次 {CurrentWaveCount} " (Variables|Default|GetCurrentWave)))
      (if (== (Variables|Default|GetCurrentWave) (Variables|Default|GetTotalWavesToSpawn))
        (Variables|Default|SetSpawnEnemyDelayTime 2.0)
        (Utilities|FlowControl|Delay 1.0)
        (CallFunction|CreateWaveWidget "最后一波")))
    (:WaveCompleted
      (CallFunction|CreateWaveWidgetCountDown (Utilities|Text|FormatText "当前来袭波次 {CurrentWaveCount} 已被击败" (Variables|Default|GetCurrentWave)) (Variables|Default|GetWaveCompletedWaitTime)))
    (:AllWavesCompleted
      (bind (_outloadeddifficulty _returnvalue) (Class|ArcaneBlueprintFunctionLibrary|TryLoadSavedGameDifficulty))
      (if _returnvalue
        (Class|ArcaneBlueprintFunctionLibrary|SaveUnlockedGameDifficulties (Utilities|Select :Index _outloadeddifficulty :None "Normal" :Easy "Normal" :Normal "Hard" :Hard "Insane" :Insane "Insane")))
      (Utilities|FlowControl|Delay 1.5)
      (CameraFades|StartCameraFade :self (Game|GetPlayerCameraManager 0) :ToAlpha 1.0 :Duration 3.0 :bHoldWhenFinished true)
      (Utilities|FlowControl|Delay 3.0)
      (Game|SetGamePaused true)
      (bind _buttontype (|PushModalScreen "(TagName=\"Frontend.Widget.ModalScreen.PlayerWin\")" "YesNoClose" "恭喜通关" (|GenerictoText (Class|KismetMathLibrary|GetDate (Math|DateTime|Now))) "得  胜" "此时重一去  去合到三清" (Variables|Default|GetWin%20Modal%20Icon) "WarningTheme" "再玩一次" "返回主菜单" "退出游戏")
        (:OnModalScreenButtonClicked
          (switch Utilities|FlowControl|Switch|SwitchonEModalButtonType _buttontype
            (:Confirm
              (Game|OpenLevel(byObjectReference) (Class|ArcaneGameInstance|GetLevelWorldbyTag (Class|ArcaneBlueprintFunctionLibrary|GetArcaneGameInstance) "(TagName=\"GameData.Level.SurvivalGameModeMap\")")))
            (:Cancel
              (Game|OpenLevel(byObjectReference) (Class|ArcaneGameInstance|GetLevelWorldbyTag (Class|ArcaneBlueprintFunctionLibrary|GetArcaneGameInstance) "(TagName=\"GameData.Level.MainMenuMap\")")))
            (:Close
              (Class|ArcaneBlueprintFunctionLibrary|ArcaneCloseGame))))))
    (:PlayerDied
      (Utilities|FlowControl|Delay 1.85)
      (CameraFades|StartCameraFade :self (Game|GetPlayerCameraManager 0) :ToAlpha 1.0 :Duration 2.0 :bHoldWhenFinished true)
      (Utilities|FlowControl|Delay 2.0)
      (Game|SetGamePaused true)
      (bind _buttontype_2 (|PushModalScreen "(TagName=\"Frontend.Widget.ModalScreen.PlayerDie\")" "YesNoClose" "" "" "死  亡" "昨夜龙湫风雨 门前石浪掀舞    四更山鬼吹灯啸 惊倒世间儿女" "(TintColor=(SpecifiedColor=(R=1.000000,G=1.000000,B=1.000000,A=1.000000),ColorUseRule=UseColor_Specified),DrawAs=Image,Tiling=NoTile,Mirroring=NoMirror,ImageType=NoImage,ImageSize=(X=32.000000,Y=32.000000),Margin=(Left=0.000000,Top=0.000000,Right=0.000000,Bottom=0.000000),ResourceObject=None,OutlineSettings=(CornerRadii=(X=0.000000,Y=0.000000,Z=0.000000,W=0.000000),Color=(SpecifiedColor=(R=0.000000,G=0.000000,B=0.000000,A=0.000000),ColorUseRule=UseColor_Specified),Width=0.000000,RoundingType=HalfHeightRadius,bUseBrushTransparency=False),UVRegion=(Min=(X=0.000000,Y=0.000000),Max=(X=0.000000,Y=0.000000),bIsValid=False),bIsDynamicallyLoaded=False,ResourceName=\"\")" "ErrorTheme" "再试一次" "返回主菜单" "退出游戏")
        (:OnModalScreenButtonClicked
          (switch Utilities|FlowControl|Switch|SwitchonEModalButtonType _buttontype_2
            (:Confirm
              (Game|OpenLevel(byObjectReference) (Class|ArcaneGameInstance|GetLevelWorldbyTag (Class|ArcaneBlueprintFunctionLibrary|GetArcaneGameInstance) "(TagName=\"GameData.Level.SurvivalGameModeMap\")")))
            (:Cancel
              (Game|OpenLevel(byObjectReference) (Class|ArcaneGameInstance|GetLevelWorldbyTag (Class|ArcaneBlueprintFunctionLibrary|GetArcaneGameInstance) "(TagName=\"GameData.Level.MainMenuMap\")")))
            (:Close
              (Class|ArcaneBlueprintFunctionLibrary|ArcaneCloseGame))))))))

(event EventBeginPlay
  (Audio|SpawnSound2D "/Game/Blueprints/Game/Audio/InGameMusic_LOOP_6_Cue.InGameMusic_LOOP_6_Cue" 1.0 1.0 0.0 0)
  (EventDispatchers|AssignOnSurvialGameModeStateChanged (delegate Custom|OnSurvialGameModeStateChangedEvent)))

(event EventTick
  (params (DeltaSeconds :type Float%20%28single-precision%29)))

(fn ConstructionScript)

(fn CreateWaveWidgetCountDown
  (params (TextOfState :type Text) (TotalCountDownTime :type Float%20%28double-precision%29))
  (bind _returnvalue (UserInterface|CreateWidget "/Game/Blueprints/UI/Widgets/GameModeWidget/WBP_WaveTextWithCountDown.WBP_WaveTextWithCountDown_C"))
  (UserInterface|Viewport|AddtoViewport _returnvalue 0)
  (Rendering|Components|TextRender|SetText (Variables|/Game/Blueprints/UI/Widgets/GameModeWidget/WBP_WaveTextWithCountDown.WBP_WaveTextWithCountDown_C|GetTextBlock_WaveText _returnvalue) TextOfState)
  (Default|StartCountDown _returnvalue TotalCountDownTime))

(fn CreateWaveWidget
  (params (WaveText :type Text))
  (bind _returnvalue (UserInterface|CreateWidget "/Game/Blueprints/UI/Widgets/GameModeWidget/WBP_WaveTextCount.WBP_WaveTextCount_C"))
  (UserInterface|Viewport|AddtoViewport _returnvalue 0)
  (Rendering|Components|TextRender|SetText (Variables|/Game/Blueprints/UI/Widgets/GameModeWidget/WBP_WaveTextCount.WBP_WaveTextCount_C|GetTextBlock_Count _returnvalue) WaveText))