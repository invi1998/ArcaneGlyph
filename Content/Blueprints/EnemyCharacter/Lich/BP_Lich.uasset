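; BP_Lich is the Lich enemy character, whose Blueprint logic handles its dissolve when it dies.
; On death it async-loads a Niagara effect, attaches it to the mesh and tints it with the material's dissolve edge color.
; A timeline scaled to the total dissolve time fades the body and both equipped weapons, then destroys them and the character.
; If the effect fails to cast, the character is destroyed immediately.
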(event EventBeginPlay
  (|CallParentFunction) ; 此节点被禁用，将不会被调用。\n从引脚连出引线来编译功能。
)

(event Collision|EventActorBeginOverlap
  (params (OtherActor :type Actor%20Object%20Reference))
  (|CallParentFunction OtherActor) ; 此节点被禁用，将不会被调用。\n从引脚连出引线来编译功能。
)

(event EventTick
  (params (DeltaSeconds :type Float%20%28single-precision%29))
  (|CallParentFunction DeltaSeconds) ; 此节点被禁用，将不会被调用。\n从引脚连出引线来编译功能。
)

(event EventOnEnemyDeath
  (bind _enemycombatcomponent (Variables|Default|GetEnemyCombatComponent))
  (bind _enemycombatcomponent_2 (Variables|Default|GetEnemyCombatComponent))
  (bind _enemycombatcomponent_3 (Variables|Default|GetEnemyCombatComponent))
  (bind _enemycombatcomponent_4 (Variables|Default|GetEnemyCombatComponent))
  (bind _mesh (Variables|Character|GetMesh))
  (bind _returnvalue (Class|PawnCombatComponent|GetCharacterCurrentEquippedWeapon _enemycombatcomponent_2 false))
  (bind _returnvalue_2 (Class|PawnCombatComponent|GetCharacterCurrentEquippedWeapon _enemycombatcomponent_3 true))
  (bind _returnvalue_3 (Class|PawnCombatComponent|GetCharacterCurrentEquippedWeapon _enemycombatcomponent false))
  (bind _returnvalue_4 (Class|PawnCombatComponent|GetCharacterCurrentEquippedWeapon _enemycombatcomponent_4 true))
  (bind _object (Utilities|AsyncLoadAsset (Variables|Default|GetDissolveNiagaraSystem))
    (:Completed
      (bind _asniagara系统 (Utilities|Casting|CastToNiagaraSystem _object)
        (:then
          (bind _returnvalue_5 (Niagara|SpawnSystemAttached _asniagara系统 (Variables|Character|GetMesh) "None" "0, 0, 0" "0, 0, 0" "KeepRelativeOffset" true))
          (bind _returnvalue_6 (Rendering|Material|CreateDynamicMaterialInstance _mesh 0 (Rendering|Material|GetMaterial _mesh 0) "None" :!class /Script/Engine.PrimitiveComponent))
          (bind _returnvalue_7 (Rendering|Material|GetVectorParameterValue _returnvalue_6 "DissolveEdgeColor" :!class /Script/Engine.MaterialInstanceDynamic))
          (Niagara|SetNiagaraVariable(LinearColor) _returnvalue_5 "DissolveParticleColor" _returnvalue_7)
          (Components|Timeline|SetPlayRate (Variables|Default|GetDissolveTimelineLich) (/ 1.0 (Variables|Default|GetTotalDissolveTime)))
          (bind (_direction _normallizedflottrack _weapontrack) (Timeline|DissolveTimelineLich PlayFromStart)
            (:Update
              (Rendering|Material|SetScalarParameterValueonMaterials (Variables|Character|GetMesh) "Dissolve" _normallizedflottrack)
              (Utilities|FlowControl|Sequence
                (:then_0
                  (Utilities|IsValid _returnvalue_3
                    (:Is%20Valid
                      (Rendering|Material|SetScalarParameterValueonMaterials (Variables|/Script/ArcaneGlyph.ArcaneWeaponBase|GetWeaponMesh _returnvalue_3) "DissolveAmount" _weapontrack))))
                (:then_1
                  (Utilities|IsValid _returnvalue_4
                    (:Is%20Valid
                      (Rendering|Material|SetScalarParameterValueonMaterials (Variables|/Script/ArcaneGlyph.ArcaneWeaponBase|GetWeaponMesh _returnvalue_4) "DissolveAmount" _weapontrack))))))
            (:Finished
              (Utilities|FlowControl|Sequence
                (:then_0
                  (Utilities|IsValid _returnvalue
                    (:Is%20Valid
                      (Actor|DestroyActor _returnvalue))))
                (:then_1
                  (Utilities|IsValid _returnvalue_2
                    (:Is%20Valid
                      (Actor|DestroyActor _returnvalue_2))))
                (:then_2
                  (Actor|DestroyActor))))))
        (:CastFailed
          (Actor|DestroyActor))))))

(fn ConstructionScript
  (|CallParentFunction))