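; Base enemy character Blueprint that handles enemy entry, death and teleport visuals plus floating combat text.
; BeginPlay spawns and binds combat text to damage dealt, reverses a dissolve on mesh and weapon, and plays a random entry montage.
; Death disables collision, clears UI, dissolves with async-loaded Niagara tinted from the material, triggers the soul-spawn ability, then destroys itself.
; Teleport events toggle dissolve instantly and spawn Niagara at a line-traced point.
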(event Custom|TeleportStart
  (bind _position (CallFunction|GetNiagaraSpawnPosition))
  (Niagara|SpawnSystematLocation (Variables|Default|GetEnterTeleport) _position "0, 0, 0" (Variables|Default|GetScaleNiagara))
  (Rendering|Material|SetScalarParameterValueonMaterials (Variables|Character|GetMesh) "DissolveAmount" 1.0))

(event Custom|TeleportEnd
  (bind _position (CallFunction|GetNiagaraSpawnPosition))
  (Niagara|SpawnSystematLocation (Variables|Default|GetEnd_Teleport) _position "0, 0, 0" (Variables|Default|GetScaleNiagara))
  (Rendering|Material|SetScalarParameterValueonMaterials (Variables|Character|GetMesh) "DissolveAmount" 0.0))

(event Custom|OnCauseDamage
  (params (InHitImpactLocation :type Vector) (InDamageValue :type Integer) (bIsCriticalHit :type Boolean))
  (CallFunction|ActivateCombatText "NewEnumerator24" 0 (Math|Conversions|ToFloat(Integer) InDamageValue) InHitImpactLocation))

(event EventBeginPlay
  (bind _entry_anim_montage (Variables|Default|GetEntry%20Anim%20Montage))
  (bind _enemycombatcomponent (Variables|Default|GetEnemyCombatComponent))
  (bind _returnvalue (Class|PawnCombatComponent|GetCharacterCurrentEquippedWeapon _enemycombatcomponent false))
  (Utilities|FlowControl|Sequence
    (:then_0
      (bind _returnvalue_2 (Game|SpawnActorfromClass "/Game/DynamicCombatText/Blueprints/BP_CombatText.BP_CombatText_C" (Math|Transform|MakeTransform "0, 0, 0") "Undefined" "OverrideRootScale" 0 0))
      (bind _output_get (Variables|Default|SetCombatText _returnvalue_2))
      (Default|Initialise _output_get self "0, 0,175.000000")
      (EventDispatchers|AssignOnCauseDamage (Variables|Default|GetEnemyCombatComponent) (delegate Custom|OnCauseDamage)))
    (:then_1
      (Components|Timeline|SetPlayRate (Variables|Default|GetEntryRestoreTimeline) (/ 1.0 (Variables|Default|GetTotalEntryRestoreTime)))
      (bind _normallizedflottrack (Timeline|EntryRestoreTimeline ReverseFromEnd)
        (:Update
          (Rendering|Material|SetScalarParameterValueonMaterials (Variables|Character|GetMesh) "DissolveAmount" _normallizedflottrack)
          (Utilities|IsValid _returnvalue
            (:Is%20Valid
              (Rendering|Material|SetScalarParameterValueonMaterials (Variables|/Script/ArcaneGlyph.ArcaneWeaponBase|GetWeaponMesh _returnvalue) "DissolveAmount" _normallizedflottrack))))))
    (:then_2
      (if (not (Utilities|Array|IsEmpty _entry_anim_montage))
        (Animation|PlayAnimMontage (.OutItem (Utilities|Array|Random _entry_anim_montage)) 1.0 "None")))))

(event Collision|EventActorBeginOverlap
  (params (OtherActor :type Actor%20Object%20Reference)))

(event EventTick
  (params (DeltaSeconds :type Float%20%28single-precision%29)))

(event EventOnEnemyDeathBegin
  (Collision|SetCollisionEnabled (Variables|Default|GetCapsuleComponent) "NoCollision"))

(event EventOnEnemyDeath
  (bind _enemycombatcomponent (Variables|Default|GetEnemyCombatComponent))
  (bind _enemycombatcomponent_2 (Variables|Default|GetEnemyCombatComponent))
  (bind _mesh (Variables|Character|GetMesh))
  (bind _returnvalue (Class|PawnCombatComponent|GetCharacterCurrentEquippedWeapon _enemycombatcomponent false))
  (bind _returnvalue_2 (Class|PawnCombatComponent|GetCharacterCurrentEquippedWeapon _enemycombatcomponent_2 false))
  (Utilities|FlowControl|Sequence
    (:then_0
      (Class|EnemyUIComponent|RemoveAllEnemyDrawnWidget (Variables|Default|GetEnemyUIComponent)))
    (:then_1
      (bind _object (Utilities|AsyncLoadAsset (Variables|Default|GetDissolveNiagaraSystem))
        (:Completed
          (bind _asniagara系统 (Utilities|Casting|CastToNiagaraSystem _object))
          (bind _returnvalue_3 (Niagara|SpawnSystemAttached _asniagara系统 (Variables|Character|GetMesh) "None" "0, 0, 0" "0, 0, 0" "KeepRelativeOffset" true))
          (bind _returnvalue_4 (Rendering|Material|CreateDynamicMaterialInstance _mesh 0 (Rendering|Material|GetMaterial _mesh 0) "None" :!class /Script/Engine.PrimitiveComponent))
          (bind _returnvalue_5 (Rendering|Material|GetVectorParameterValue _returnvalue_4 "DissolveEdgeColor" :!class /Script/Engine.MaterialInstanceDynamic))
          (Niagara|SetNiagaraVariable(LinearColor) _returnvalue_3 "DissolveParticleColor" _returnvalue_5)
          (Components|Timeline|SetPlayRate (Variables|Default|GetDissolveTimeline) (/ 1.0 (Variables|Default|GetTotalDissolveTime)))
          (bind _normallizedflottrack (Timeline|DissolveTimeline PlayFromStart)
            (:Update
              (Rendering|Material|SetScalarParameterValueonMaterials (Variables|Character|GetMesh) "DissolveAmount" _normallizedflottrack)
              (Utilities|IsValid _returnvalue
                (:Is%20Valid
                  (Rendering|Material|SetScalarParameterValueonMaterials (Variables|/Script/ArcaneGlyph.ArcaneWeaponBase|GetWeaponMesh _returnvalue) "DissolveAmount" _normallizedflottrack))))
            (:Finished
              (Utilities|FlowControl|Sequence
                (:then_0
                  (Utilities|IsValid _returnvalue_2
                    (:Is%20Valid
                      (Actor|DestroyActor _returnvalue_2))))
                (:then_1
                  (Class|ArcaneAbilitySystemComponent|TryActivateAbilitybyTag (Variables|Default|GetArcaneAbilitySystemComponent) "(TagName=\"Enemy.Ability.SpawnSoul\")")
                  (Utilities|FlowControl|Delay 0.2)
                  (Actor|DestroyActor))))))))))

(fn ConstructionScript
  (Rendering|Material|SetVectorParameterValueonMaterials (Variables|Character|GetMesh) "Color" (Variables|Default|GetColor%20Teleport)))

(fn GetNiagaraSpawnPosition
  (bind _returnvalue (Transformation|GetActorLocation))
  (bind _outhit (Collision|LineTraceForObjects _returnvalue (+ _returnvalue (* (Transformation|GetActorUpVector) (Variables|Default|GetTraceLength))) (Variables|Default|GetObject%20Types) false 0 "None"))
  (return (.ImpactPoint (Collision|BreakHitResult _outhit))))

(fn ActivateCombatText
  (params (TextType :type ENUM_TextTypes%20Enum :default "NewEnumerator0") (TextSubTypeIndex :type Integer) (Damage :type Float%20%28double-precision%29) (ImpactPoint :type Vector))
  (LocalVariables|SetTextType_Local TextType)
  (LocalVariables|SetTextSubType_Local TextSubTypeIndex)
  (LocalVariables|SetDamage_Local Damage)
  (LocalVariables|SetImpactPoint_Local ImpactPoint)
  (switch Utilities|FlowControl|Switch|SwitchonENUM_TextTypes (LocalVariables|GetTextType_Local)
    (:NewEnumerator0
      ;[1 1 1] Normal damage
      (Default|ActivateText (Variables|Default|GetCombatText) "NewEnumerator0" (LocalVariables|GetDamage_Local) true (LocalVariables|GetImpactPoint_Local)))
    (:NewEnumerator1
      ;[1 1 1] Critical Hit Damage
      (Default|ActivateText (Variables|Default|GetCombatText) "NewEnumerator1" (LocalVariables|GetDamage_Local) true (LocalVariables|GetImpactPoint_Local)))
    (:NewEnumerator14
      (switch int (LocalVariables|GetTextSubType_Local)
        (:0
          ;[1 1 1] Stun
          (Default|ActivateTextwithOverrides (Variables|Default|GetCombatText) "NewEnumerator14" 0.0 true (LocalVariables|GetImpactPoint_Local) true "STUN" true "(R=0.786458,G=0.050748,B=0.144906,A=1.000000)" false 0 true "(R=0.062500,G=0.005825,B=0.007692,A=1.000000)" false "(R=0.000000,G=0.000000,B=0.000000,A=1.000000)"))
        (:1
          ;[1 1 1] Slow
          (Default|ActivateTextwithOverrides (Variables|Default|GetCombatText) "NewEnumerator14" 0.0 true (LocalVariables|GetImpactPoint_Local) true "SLOW" true "(R=0.921875,G=0.683376,B=0.045696,A=1.000000)" false 0 true "(R=0.083333,G=0.067189,B=0.004680,A=1.000000)" false "(R=0.000000,G=0.000000,B=0.000000,A=1.000000)"))
        (:2
          ;[1 1 1] Silence
          (Default|ActivateTextwithOverrides (Variables|Default|GetCombatText) "NewEnumerator14" 0.0 true (LocalVariables|GetImpactPoint_Local) true "SILENCE" true "(R=0.044310,G=0.305868,B=0.468750,A=1.000000)" false 0 true "(R=0.011227,G=0.052698,B=0.067708,A=1.000000)" false "(R=0.000000,G=0.000000,B=0.000000,A=1.000000)"))
        (:3
          ;[1 1 1] Confuse
          (Default|ActivateTextwithOverrides (Variables|Default|GetCombatText) "NewEnumerator14" 0.0 true (LocalVariables|GetImpactPoint_Local) true "CONFUSE" true "(R=0.927083,G=0.018852,B=0.693504,A=1.000000)" false 0 true "(R=0.055738,G=0.007898,B=0.057292,A=1.000000)" false "(R=0.000000,G=0.000000,B=0.000000,A=1.000000)"))))
    (:NewEnumerator21
      (switch int (LocalVariables|GetTextSubType_Local)
        (:0
          ;[1 1 1] Block
          (Default|ActivateTextwithOverrides (Variables|Default|GetCombatText) "NewEnumerator21" 0.0 true (LocalVariables|GetImpactPoint_Local) true "BLOCK" false "(R=0.000000,G=0.000000,B=0.000000,A=1.000000)" false 0 false "(R=0.000000,G=0.000000,B=0.000000,A=1.000000)" false "(R=0.000000,G=0.000000,B=0.000000,A=1.000000)"))
        (:1
          ;[1 1 1] Evade
          (Default|ActivateTextwithOverrides (Variables|Default|GetCombatText) "NewEnumerator21" 0.0 true (LocalVariables|GetImpactPoint_Local) true "EVADE" false "(R=0.000000,G=0.000000,B=0.000000,A=1.000000)" false 0 false "(R=0.000000,G=0.000000,B=0.000000,A=1.000000)" false "(R=0.000000,G=0.000000,B=0.000000,A=1.000000)"))
        (:2
          ;[1 1 1] Parry
          (Default|ActivateTextwithOverrides (Variables|Default|GetCombatText) "NewEnumerator21" 0.0 true (LocalVariables|GetImpactPoint_Local) true "PARRY" false "(R=0.000000,G=0.000000,B=0.000000,A=1.000000)" false 0 false "(R=0.000000,G=0.000000,B=0.000000,A=1.000000)" false "(R=0.000000,G=0.000000,B=0.000000,A=1.000000)"))
        (:3
          ;[1 1 1] Absorb
          (Default|ActivateTextwithOverrides (Variables|Default|GetCombatText) "NewEnumerator21" 0.0 true (LocalVariables|GetImpactPoint_Local) true "ABSORB" false "(R=0.000000,G=0.000000,B=0.000000,A=1.000000)" false 0 false "(R=0.000000,G=0.000000,B=0.000000,A=1.000000)" false "(R=0.000000,G=0.000000,B=0.000000,A=1.000000)"))))
    (:NewEnumerator23
      (switch int (LocalVariables|GetTextSubType_Local)
        (:0
          ;[1 1 1] Fire
          (Default|ActivateTextwithOverrides (Variables|Default|GetCombatText) "NewEnumerator23" (LocalVariables|GetDamage_Local) true (LocalVariables|GetImpactPoint_Local) true "Burn" true "(R=0.692708,G=0.234298,B=0.030984,A=1.000000)" true "/Game/DynamicCombatText/Textures/T_FireIcon.T_FireIcon" false "(R=0.000000,G=0.000000,B=0.000000,A=1.000000)" false "(R=0.000000,G=0.000000,B=0.000000,A=1.000000)"))
        (:1
          ;[1 1 1] Poison
          (Default|ActivateTextwithOverrides (Variables|Default|GetCombatText) "NewEnumerator23" (LocalVariables|GetDamage_Local) true (LocalVariables|GetImpactPoint_Local) true "Poison" true "(R=0.037627,G=0.692708,B=0.250169,A=1.000000)" true "/Game/DynamicCombatText/Textures/T_PoisonIcon.T_PoisonIcon" false "(R=0.000000,G=0.000000,B=0.000000,A=1.000000)" false "(R=0.000000,G=0.000000,B=0.000000,A=1.000000)"))
        (:2
          ;[1 1 1] Cold
          (Default|ActivateTextwithOverrides (Variables|Default|GetCombatText) "NewEnumerator23" (LocalVariables|GetDamage_Local) true (LocalVariables|GetImpactPoint_Local) true "Cold" true "(R=0.013630,G=0.500073,B=0.833333,A=1.000000)" true "/Game/DynamicCombatText/Textures/T_IceIcon.T_IceIcon" false "(R=0.000000,G=0.000000,B=0.000000,A=1.000000)" false "(R=0.000000,G=0.000000,B=0.000000,A=1.000000)"))
        (:3
          ;[1 1 1] Electric
          (Default|ActivateTextwithOverrides (Variables|Default|GetCombatText) "NewEnumerator23" (LocalVariables|GetDamage_Local) true (LocalVariables|GetImpactPoint_Local) true "Shock" true "(R=0.692708,G=0.586732,B=0.209256,A=1.000000)" true "/Game/DynamicCombatText/Textures/T_LightningIcon.T_LightningIcon" false "(R=0.000000,G=0.000000,B=0.000000,A=1.000000)" false "(R=0.000000,G=0.000000,B=0.000000,A=1.000000)"))))
    (:NewEnumerator24
      ;[1 1 1] Player Hit Damage
      (Default|ActivateText (Variables|Default|GetCombatText) "NewEnumerator24" (LocalVariables|GetDamage_Local) true (LocalVariables|GetImpactPoint_Local)))))