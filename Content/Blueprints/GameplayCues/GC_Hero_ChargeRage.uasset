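; Gameplay Cue for the hero's rage charge, providing looping-state visual and audio feedback while the cue is active.
; WhileActive spawns a charging-energy Niagara system on the SpearSocket and an attached charge sound on the cue's target attach component, storing both.
; OnRemove destroys the effect component and stops and destroys the sound, guarding each with a validity check.
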(event EventBeginPlay)

(event Collision|EventActorBeginOverlap
  (params (OtherActor :type Actor%20Object%20Reference)))

(event EventTick
  (params (DeltaSeconds :type Float%20%28single-precision%29)))

(fn ConstructionScript)

(fn WhileActive
  (params (MyTarget :type Actor%20Object%20Reference) (Parameters :type Gameplay%20Cue%20Parameters%20Structure%20%28by%20ref%29))
  (Utilities|FlowControl|Sequence
    (:then_0
      (bind _returnvalue (Niagara|SpawnSystemAttached "/Game/UltraFXWarrior/FX/NiagaraSystem/Abilities/15_Heavy_Strike/NS_Heavy_Strike_01_ChargingEnergy1.NS_Heavy_Strike_01_ChargingEnergy1" (.TargetAttachComponent (Ability|GameplayCue|BreakGameplayCueParameters Parameters)) "SpearSocket" "0, 0, 0" "0, 0, 0" "KeepRelativeOffset" false))
      (Variables|Default|SetAttachedRageFX _returnvalue))
    (:then_1
      (bind _returnvalue_2 (Audio|SpawnSoundAttached "/Game/Assets/Sounds/Wukong/SC_ChargeBeans.SC_ChargeBeans" (.TargetAttachComponent (Ability|GameplayCue|BreakGameplayCueParameters Parameters)) "None" "0, 0, 0" "0, 0, 0" "KeepRelativeOffset" false 1.0 1.0 0.0 0 0))
      (Variables|Default|SetRageSound _returnvalue_2))
    (:then_2
      (return false))))

(fn OnRemove
  (params (MyTarget :type Actor%20Object%20Reference) (Parameters :type Gameplay%20Cue%20Parameters%20Structure%20%28by%20ref%29))
  (Utilities|FlowControl|Sequence
    (:then_0
      (bind _attachedragefx (Variables|Default|GetAttachedRageFX)
        (:then
          (Components|DestroyComponent _attachedragefx))
        (:else)))
    (:then_1
      (bind _ragesound (Variables|Default|GetRageSound)
        (:then
          (Audio|Components|Audio|Stop _ragesound)
          (Components|DestroyComponent _ragesound))
        (:else)))
    (:then_2
      (return false))))