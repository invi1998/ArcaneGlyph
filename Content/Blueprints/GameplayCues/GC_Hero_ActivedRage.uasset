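; Gameplay cue that provides the visual and audio feedback while a hero's rage is active.
; WhileActive spawns a burst effect at the target's root socket, attaches a persistent Niagara effect and plays a heart sound at the actor's location.
; OnRemove destroys the stored attached effect and checks RageSound for cleanup, though the sound played here is never stored in that variable.
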(event EventBeginPlay)

(event Collision|EventActorBeginOverlap
  (params (OtherActor :type Actor%20Object%20Reference)))

(event EventTick
  (params (DeltaSeconds :type Float%20%28single-precision%29)))

(fn ConstructionScript)

(fn WhileActive
  (params (MyTarget :type Actor%20Object%20Reference) (Parameters :type Gameplay%20Cue%20Parameters%20Structure%20%28by%20ref%29))
  (Utilities|FlowControl|Sequence
    (:then_0
      (Niagara|SpawnSystematLocation 0 "/Game/UltraFXWarrior/FX/NiagaraSystem/Abilities/05_Conqueror/NS_Conqueror_03_Burst.NS_Conqueror_03_Burst" (Transformation|GetSocketLocation (.TargetAttachComponent (Ability|GameplayCue|BreakGameplayCueParameters Parameters)) "root")))
    (:then_1
      (bind _returnvalue (Niagara|SpawnSystemAttached "/Game/Character_VFX_Pack/VFX/V9/NS_Character_VFX_9.NS_Character_VFX_9" (.TargetAttachComponent (Ability|GameplayCue|BreakGameplayCueParameters Parameters)) "None" "0, 0, 0" "0, 0, 0" "KeepRelativeOffset" false))
      (Variables|Default|SetAttachedRageFX _returnvalue))
    (:then_2
      (Audio|PlaySoundatLocation 0 "/Game/Assets/Sounds/A_Heart.A_Heart" (Transformation|GetActorLocation MyTarget) "0, 0, 0" 1.0 1.0 0.0 0 0 0 0))
    (:then_3
      (return false))))

(fn OnRemove
  (params (MyTarget :type Actor%20Object%20Reference) (Parameters :type Gameplay%20Cue%20Parameters%20Structure%20%28by%20ref%29))
  (Utilities|FlowControl|Sequence
    (:then_0
      (bind _attachedragefx (Variables|Default|GetAttachedRageFX)
        (:then
          (Components|DestroyComponent _attachedragefx))
        (:else)))
    (:then_1
      (bind _ragesound (Variables|Default|GetRageSound)
        (:then
          (Components|DestroyComponent _ragesound))
        (:else)))
    (:then_2
      (return false))))