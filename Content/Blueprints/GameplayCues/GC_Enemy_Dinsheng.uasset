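; Gameplay cue that freezes an enemy Character in place and outlines it while the cue is active.
; WhileActive sets the target's CustomTimeDilation to zero and applies an outline overlay material to its mesh.
; OnRemove clears the overlay and restores normal time dilation.
; Both call the parent handler, though WhileActive skips it when the target is not a Character.
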(fn WhileActive
  (params (MyTarget :type Actor%20Object%20Reference) (Parameters :type Gameplay%20Cue%20Parameters%20Structure%20%28by%20ref%29))
  (bind _as角色 (Utilities|Casting|CastToCharacter MyTarget))
  (Variables|/Script/Engine.Actor|SetCustomTimeDilation _as角色 0.0)
  (Rendering|Material|SetOverlayMaterial (Variables|/Script/Engine.Character|GetMesh _as角色) "/Game/OverlayOutlineM/Material/MI_Outline_6_Inst.MI_Outline_6_Inst" :!class /Script/Engine.MeshComponent)
  (return (|CallParentFunction MyTarget Parameters)))

(fn OnRemove
  (params (MyTarget :type Actor%20Object%20Reference) (Parameters :type Gameplay%20Cue%20Parameters%20Structure%20%28by%20ref%29))
  (bind _as角色 (Utilities|Casting|CastToCharacter MyTarget)
    (:then
      (Rendering|Material|SetOverlayMaterial (Variables|/Script/Engine.Character|GetMesh _as角色) 0 :!class /Script/Engine.MeshComponent)
      (Variables|/Script/Engine.Actor|SetCustomTimeDilation _as角色 1.0)
      (return (|CallParentFunction MyTarget Parameters)))
    (:CastFailed
      (return (|CallParentFunction MyTarget Parameters)))))